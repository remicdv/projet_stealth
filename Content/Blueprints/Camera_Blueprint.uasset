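; Security camera that sweeps back and forth and alerts every IA_BluePrint AI with its light's position when its Cone overlaps the player.
; Tick reverses pitch rotation on a real-time cycle and drives a PointLight showing red on detection.
; Once Seized, the light stays visible, yellow when clear.
; Setting Control then turns on Interrupteur for a few seconds; while Seized, this turns the light green and suppresses detection.
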(event Custom|CloseCameraOff
  (Variables|Default|SetInterrupteur false))

(event EventTick
  (params (DeltaSeconds :type Float%20%28single-precision%29))
  (bind _cone (Variables|Default|GetCone))
  (bind _mainc (Variables|Default|GetMainC))
  (bind _pointlight (Variables|Default|GetPointLight))
  (bind _pointlight_2 (Variables|Default|GetPointLight))
  (bind _seized (Variables|Default|GetSeized))
  (bind _returnvalue (Collision|IsOverlappingActor _cone _mainc :!class /Script/Engine.PrimitiveComponent))
  (Utilities|FlowControl|Sequence
    (:then_0
      ;[1 1 1] Gestion des booléens : Seized = Le control Pannel a été pris par le joueur, Control = Le joueur a pris possession de la caméra, Collision = Le joueur est dans le champ de vision de la caméra et pas la posession
      (Rendering|SetVisibility (Variables|Default|GetPointLight) _returnvalue false)
      (if _seized
        (Rendering|SetVisibility (Variables|Default|GetPointLight) _seized false)
        (if (Variables|Default|GetInterrupteur)
          (Rendering|Components|Light|SetLightColor _pointlight_2 "(R=0.009027,G=1.000000,B=0.000000,A=1.000000)" true)
          (Variables|Default|SetCamera_Collision false :!label _label)
          (elif _returnvalue
            (Rendering|Components|Light|SetLightColor _pointlight "(R=1.000000,G=0.000000,B=0.000000,A=1.000000)" true :!label _label_2)
            (Variables|Default|SetCamera_Collision _returnvalue)
            (else
              (Rendering|Components|Light|SetLightColor _pointlight_2 "(R=1.000000,G=0.837452,B=0.000000,A=1.000000)" true)
              (goto _label))))
        (else
          (goto _label_2))))
    (:then_1
      (if (Variables|Default|GetCamera_Collision)
        (bind _outactors (Actor|GetAllActorsOfClass "/Game/Blueprints/IA_Blueprint/IA/IA_BluePrint.IA_BluePrint_C"))
        (for _array_element _outactors
          (Utilities|FlowControl|Sequence
            (:then_0
              (Variables|/Game/Blueprints/IA_Blueprint/IA/IA_BluePrint.IA_BluePrint_C|Setposition%20camera _array_element (Transformation|GetWorldLocation _pointlight)))
            (:then_1
              (Variables|/Game/Blueprints/IA_Blueprint/IA/IA_BluePrint.IA_BluePrint_C|Setboolean%20camera _array_element true))))))
    (:then_2
      ;[1 1 1] Gestion de la rotation de la Caméra
      (bind _output_get (Variables|Default|SetTurn (> (Math|Float|%(Float) (Utilities|Time|GetRealTimeSeconds) 1e+01) 5.0)))
      (if _output_get
        (Variables|Default|SetTurnValue 1.0)
        (else
          (Variables|Default|SetTurnValue -1.0)))
      (Transformation|AddActorLocalRotation (Math|Rotator|MakeRotator 0.0 (* DeltaSeconds (Math|Float|MakeLiteralFloat 15.0) (Variables|Default|GetTurnValue)) 0.0) false false))
    (:then_3
      (if (Variables|Default|GetControl)
        (Variables|Default|SetControl false)
        (Variables|Default|SetInterrupteur true)
        (Utilities|Time|SetTimerbyEvent (delegate Custom|CloseCameraOff) 5.0)))))

(event EventBeginPlay
  ;[1 1 1] On Set l'attribut MainC au personnage controllé pour les collisions
  (Utilities|FlowControl|Sequence
    (:then_0
      (bind _asfirst_person_character (Utilities|Casting|CastToFirstPersonCharacter (Game|GetPlayerCharacter 0)))
      (Variables|Default|SetMainC _asfirst_person_character))))

(fn ConstructionScript)